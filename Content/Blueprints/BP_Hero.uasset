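; Player hero Blueprint with a three-swing sword combo, health, health kit use and save-game persistence.
; Attack input plays montages in sequence, using combo window events and input buffering, with a timer reset after the final swing.
; Enabling the weapon collider triggers global slow-motion hit-stop, then delayed collision shutoff; overlaps deal damage.
; BeginPlay restores HP, score and inventory and creates the HUD; using a kit heals and saves.
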(event `OnComboWindowClose`
  (if (`self.bCanCombo`)
    (`self.ResetCombo`)))

(event `OnComboWindowOpen`
  (bind _combocounter (`self.ComboCounter`))
  (set `self.bCanCombo` true)
  (if (`self.bAttackBuffered`)
    (`KismetSystemLibrary.K2_ClearAndInvalidateTimerHandle` (`self.ComboTimer`) :!label _label)
    (if (== (`self.ComboCounter`) 0)
      (`self.PlayAnimMontage` (select `int` (`self.ComboCounter`) :`0` "/Game/UAL2_Standard/Retarget/UAL2_StandardSword_Regular_A_Montage.UAL2_StandardSword_Regular_A_Montage" :`1` "/Game/UAL2_Standard/Retarget/UAL2_StandardSword_Regular_B_Montage.UAL2_StandardSword_Regular_B_Montage" :`2` "/Game/UAL2_Standard/Retarget/UAL2_StandardSword_Regular_C_Montage.UAL2_StandardSword_Regular_C_Montage" :!type "AnimMontage Object Reference") :!label _label_2)
      (set `self.bCanCombo` false)
      (set `self.bAttackBuffered` false)
      (`/Engine/EditorBlueprintResources/StandardMacros.IncrementInt` _combocounter
        (:`  `
          (if (> _combocounter 2)
            (bind _returnvalue (`KismetSystemLibrary.K2_SetTimer` null "ResetCombo" 0.8))
            (set `self.ComboTimer` _returnvalue))))
      (elif (`self.bCanCombo`)
        (goto _label_2)
        (else
          (set `self.bAttackBuffered` true))))))

(event `EnhancedInput|/Game/Input/IA_Attack`
  (params (ActionValue :type Boolean) (ElapsedSeconds :type "Float (double-precision)") (TriggeredSeconds :type "Float (double-precision)") (InputAction :type "InputAction Object Reference" :default "/Game/Input/IA_Attack.IA_Attack"))
  (:`Started`
    (if (not (> (`self.ComboCounter`) 2))
      (goto _label))))

(event `DisableWeaponCollision`
  (`PrimitiveComponent.SetCollisionEnabled` (`self.WeaponCollider`) "NoCollision"))

(event `EnableWeaponCollision`
  (`PrimitiveComponent.SetCollisionEnabled` (`self.WeaponCollider`) "QueryOnly")
  (`GameplayStatics.SetGlobalTimeDilation` 0.05)
  (`Timeline|HitStopTimeline` :!via `PlayFromStart`
    (:`Finished`
      (`GameplayStatics.SetGlobalTimeDilation` 1.0)
      (`KismetSystemLibrary.K2_SetTimer` null "DisableWeaponCollision" 0.3))))

(event `self.ReceiveAnyDamage`
  (params (Damage :type "Float (single-precision)") (DamageType :type "DamageType Object Reference") (InstigatedBy :type "Controller Object Reference") (DamageCauser :type "Actor Object Reference"))
  (set `self.Hp` (- (`self.Hp`) Damage)))

(event `self.ReceiveBeginPlay`
  (`GameplayStatics.DoesSaveGameExist` "PRCSave Game")
  (if true
    (bind _returnvalue (`GameplayStatics.LoadGameFromSlot` "PRCSave Game"))
    (bind _asprcsave_game (cast `PRCSaveGame` _returnvalue))
    (set `self.Hp` (`PRCSaveGame.HP` _asprcsave_game))
    (set `self.Score` (`PRCSaveGame.Score` _asprcsave_game))
    (set `InventoryComponent.Items` (`PRCSaveGame.Inventory` _asprcsave_game) (`self.Inventory`)))
  (`PrimitiveComponent.SetCollisionEnabled` (`self.WeaponCollider`) "NoCollision")
  (bind _returnvalue_2 (`|CreateWidget` "/Game/Blueprints/WBP_HUD.WBP_HUD_C"))
  (`UserWidget.AddToViewport` _returnvalue_2 0))

(event `self.WeaponCollider.OnComponentBeginOverlap`
  (params (OverlappedComponent :type "PrimitiveComponent Object Reference") (OtherActor :type "Actor Object Reference") (OtherComp :type "PrimitiveComponent Object Reference") (OtherBodyIndex :type Integer) (bFromSweep :type Boolean) (SweepResult :type "HitResult Structure (by ref)"))
  (if (not (== OtherActor self))
    (`GameplayStatics.ApplyDamage` OtherActor 20.0)))

(event `EnhancedInput|/Game/Input/IA_UseItem`
  (params (ActionValue :type Boolean) (ElapsedSeconds :type "Float (double-precision)") (TriggeredSeconds :type "Float (double-precision)") (InputAction :type "InputAction Object Reference" :default "/Game/Input/IA_UseItem.IA_UseItem"))
  (:`Started`
    (bind _returnvalue (`InventoryComponent.RemoveItem` (`self.Inventory`) "HealthKit"))
    (if _returnvalue
      (set `self.Hp` (`KismetMathLibrary.FMin` (+ (`self.Hp`) 30.0) (`self.MaxHp`)))
      (`self.SaveProgress`))))

(event `SaveProgress`
  (bind _returnvalue (`GameplayStatics.CreateSaveGameObject` "/Script/PRC.PRCSaveGame"))
  (set `PRCSaveGame.Score` (`self.Score`) _returnvalue)
  (set `PRCSaveGame.HP` (`self.Hp`) _returnvalue)
  (set `PRCSaveGame.Inventory` (`InventoryComponent.Items` (`self.Inventory`)) _returnvalue)
  (`GameplayStatics.SaveGameToSlot` _returnvalue "PRCSave Game"))

(fn `ResetCombo`
  (set `self.bCanCombo` false)
  (`KismetSystemLibrary.K2_ClearAndInvalidateTimerHandle` (`self.ComboTimer`))
  (set `self.ComboCounter` 0)
  (set `self.bAttackBuffered` false))

(fn `UserConstructionScript`)