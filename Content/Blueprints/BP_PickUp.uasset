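; BP_PickUp is a collectible that grants the hero either score points or an inventory item.
; When BP_Hero overlaps its collision sphere, it plays a Niagara burst and coin sound at the hero's location.
; An empty ItemName adds PointValue to Score, while a set name adds that item to the hero's Inventory.
; Both paths save the hero's progress, then call Collect, whose logic lies outside these graphs.
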(event `self.CollisionSphere.OnComponentBeginOverlap`
  (params (OverlappedComponent :type "PrimitiveComponent Object Reference") (OtherActor :type "Actor Object Reference") (OtherComp :type "PrimitiveComponent Object Reference") (OtherBodyIndex :type Integer) (bFromSweep :type Boolean) (SweepResult :type "HitResult Structure (by ref)"))
  (bind _returnvalue (`self.K2_GetActorLocation` OtherActor))
  (bind _itemname (`self.ItemName`))
  (bind _asbp_hero (cast `/Game/Blueprints/BP_Hero` OtherActor))
  (`NiagaraFunctionLibrary.SpawnSystemAtLocation` "/Game/VFX/NS_CollectBurst.NS_CollectBurst" _returnvalue)
  (`GameplayStatics.PlaySoundAtLocation` "/Game/400_Sounds_Pack/Retro/coin.coin" _returnvalue (struct) 1.0 1.0 0.0 null null null null)
  (set `self.HERO_BP` _asbp_hero)
  (if (`KismetStringLibrary.IsEmpty` _itemname)
    (set `/Game/Blueprints/BP_Hero.Score` (`KismetMathLibrary.FTrunc` (+ (`KismetMathLibrary.Conv_IntToDouble` (`/Game/Blueprints/BP_Hero.Score` (`self.HERO_BP`))) (`self.PointValue`))) (`self.HERO_BP`))
    (`/Game/Blueprints/BP_Hero.SaveProgress` (`self.HERO_BP`))
    (`self.Collect` OtherActor)
    (else
      (`InventoryComponent.AddItem` (`/Game/Blueprints/BP_Hero.Inventory` (`self.HERO_BP`)) _itemname)
      (`/Game/Blueprints/BP_Hero.SaveProgress` (`self.HERO_BP`))
      (`self.Collect` (`self.HERO_BP`)))))

(fn `UserConstructionScript`)